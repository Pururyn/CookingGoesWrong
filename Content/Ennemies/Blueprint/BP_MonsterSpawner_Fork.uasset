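; BP_MonsterSpawner_Fork is a fork enemy that chases the player, deals contact damage and can be destroyed.
; An AI MoveTo loop re-targets the player after a short delay on success or failure.
; Damage taken updates a health bar widget and destroys the actor at zero HP.
; Capsule hits damage the player through a delayed-reset DoOnce, which stays closed if the first hit is a non-player.
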(event OnComponentHit(CapsuleComponent)
  (params (HitComponent :type Primitive%20Component%20Object%20Reference) (OtherActor :type Actor%20Object%20Reference) (OtherComp :type Primitive%20Component%20Object%20Reference) (NormalImpulse :type Vector :default "0, 0, 0") (Hit :type Hit%20Result%20Structure%20%28by%20ref%29))
  ;[0.15 0.15 0.15 0.5] Damage on player
  (Utilities|FlowControl|DoOnce false :!label _label
    (:Completed
      (bind _asbp_third_person_character (Utilities|Casting|CastToBP_ThirdPersonCharacter OtherActor))
      (Default|PlayerTakeDamage _asbp_third_person_character 2e+01)
      (Utilities|FlowControl|Delay 0.2)
      (goto _label Reset))))

(event Custom|TakeDamage
  (params (Damage :type Float%20%28double-precision%29))
  ;[0.15 0.15 0.15 0.5] Health + taking damage
  (bind _output_get (Variables|Default|SetHP (- (Variables|Default|GetHP) Damage)))
  ;[0.15 0.15 0.15 0.5] Health Bar
  (bind _aswbp_health_bar (Utilities|Casting|CastToWBP_HealthBar (UserInterface|GetUserWidgetObject (Variables|Default|GetHealthWidget))))
  (Default|UpdateHealth _aswbp_health_bar (/ _output_get 1e+02))
  (if (<= _output_get 0.0)
    (Actor|DestroyActor)))

(event EventBeginPlay
  ;[0.15 0.15 0.15 0.5] Moving Fork
  (AI|AIMoveTo self "0, 0, 0" (Game|GetPlayerCharacter 0) 5e+01 false :!label _label
    (:OnSuccess
      _)
    (:OnFail
      _))
  (Utilities|FlowControl|Delay 0.1)
  (goto _label))

(fn ConstructionScript)