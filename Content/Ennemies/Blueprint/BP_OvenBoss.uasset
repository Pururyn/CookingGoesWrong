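; BP_OvenBoss is an oven boss enemy that fires chicken projectiles toward the player.
; Every tick it rotates to face the player character using a look-at rotation, including pitch.
; A looping timer started on BeginPlay spawns BP_Projectile_Chicken at the SpawnPoint component's transform at a fixed interval.
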(event Custom|ShootChicken
  (Game|SpawnActorfromClass "/Game/Ennemies/Blueprint/BP_Projectile_Chicken.BP_Projectile_Chicken_C" (Transformation|GetWorldTransform (Variables|Default|GetSpawnPoint)) "Undefined" "MultiplyWithRoot" 0 0))

(event EventBeginPlay
  (Utilities|Time|SetTimerbyEvent (delegate Custom|ShootChicken) 3.0 true))

(event EventTick
  (params (DeltaSeconds :type Float%20%28single-precision%29))
  (Transformation|SetActorRotation (Math|Rotator|FindLookatRotation (Transformation|GetActorLocation) (Transformation|GetActorLocation (Game|GetPlayerCharacter 0)))))

(fn ConstructionScript)