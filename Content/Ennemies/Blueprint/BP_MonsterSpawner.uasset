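; BP_MonsterSpawner periodically spawns a random enemy at its own transform.
; BeginPlay starts a looping timer at SpawnInterval that fires SpawnOneMonster, which picks a class from EnnemiesToSpawn and adjusts placement on collision but always spawns.
; Spawning pauses while the level holds MaxMonster or more Character actors, a count that includes every Character, not just monsters.
; The SpawnTimer assignment is disconnected, so the timer handle is never stored.
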(event Custom|SpawnOneMonster
  (bind _ennemiestospawn (Variables|Default|GetEnnemiesToSpawn))
  ;[0.15 0.15 0.15 0.5] Count nb monster to stop spawn at max reached
  (bind _outactors (Actor|GetAllActorsOfClass "/Script/Engine.Character"))
  (if (< (Utilities|Array|Length _outactors) (Variables|Default|GetMaxMonster))
    (Game|SpawnActorfromClass (Utilities|Array|Get(acopy) _ennemiestospawn (Math|Random|RandomIntegerinRange 0 (Utilities|Array|LastIndex _ennemiestospawn))) (Transformation|GetActorTransform) "AdjustIfPossibleButAlwaysSpawn" "MultiplyWithRoot" 0 0)))

(event EventBeginPlay
  ;[0.15 0.15 0.15 0.5] Spawn Time
  (bind _returnvalue (Utilities|Time|SetTimerbyEvent (delegate Custom|SpawnOneMonster) (Variables|Default|GetSpawnInterval) true)))

(event Collision|EventActorBeginOverlap
  (params (OtherActor :type Actor%20Object%20Reference)))

(event EventTick
  (params (DeltaSeconds :type Float%20%28single-precision%29)))

(fn ConstructionScript)